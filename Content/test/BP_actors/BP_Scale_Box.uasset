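; BP_Scale_Box is a test actor whose Cube component shrinks step by step as actors overlap it.
; On overlap begin, a short delay runs, then the cube's world scale is set from the stored Scale variable.
; Scale is then reduced uniformly and printed for debugging, so the printed value is the next size to apply, one step ahead of the cube.
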(event `self.ReceiveActorBeginOverlap`
  (params (OtherActor :type "Actor Object Reference"))
  (bind _scale (`self.Scale`))
  (`KismetSystemLibrary.Delay` 0.2)
  (`SceneComponent.SetWorldScale3D` (`self.Cube`) (`self.Scale`))
  (set `self.Scale` (- _scale (0.1 0.1 0.1)))
  (`KismetSystemLibrary.PrintString` (`KismetStringLibrary.Conv_VectorToString` _scale) true true (struct :`R` 1.0 :`G` 0.743994 :`A` 1.0))
  (`parent.ReceiveActorBeginOverlap` OtherActor))

(fn `UserConstructionScript`
  (`parent.UserConstructionScript`))