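; BP_FirstActor is a test actor that flashes its SpotLight a set number of times when play begins.
; BeginPlay switches the light off, then a DoN loop capped by NumberOfFlashes feeds back into itself through delays, holding each flash for DurationOfFlashes and printing on/off.
; LightOn and LightOff set IsEnable and the spotlight's visibility.
; RotationCube adds a yaw step to the Cube, but nothing here calls it.
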(event `self.ReceiveBeginPlay`
  (`self.Light_off`)
  (`/Engine/EditorBlueprintResources/StandardMacros.Do N` (`self.number of flashes`) :!label _label
    (:`Exit`
      (`KismetSystemLibrary.Delay` 0.2)
      (`self.light_on`)
      (`KismetSystemLibrary.PrintString` "on")
      (`KismetSystemLibrary.Delay` (`self.duration of flashes`))
      (`self.Light_off`)
      (`KismetSystemLibrary.PrintString` "off")
      (goto _label))))

(event `self.ReceiveTick`
  (params (DeltaSeconds :type "Float (single-precision)")))

(fn `Light_off`
  (bind _output_get (set `self.IsEnable ` false))
  (`SceneComponent.SetVisibility` (`self.SpotLight`) _output_get false)
  (return))

(fn `light_on`
  (bind _output_get (set `self.IsEnable ` true))
  (`SceneComponent.SetVisibility` (`self.SpotLight`) _output_get false)
  (return))

(fn `RotationCube`
  (`SceneComponent.K2_AddWorldRotation` (`self.Cube`) (struct :`Pitch` 10.0) false false))

(fn `UserConstructionScript`)